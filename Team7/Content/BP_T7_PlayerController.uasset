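; Player controller Blueprint for T7 that binds five debug keys to exercise HUD and game state updates.
; One key creates a WBP_KillLog widget with placeholder names and a fixed rifle icon and adds it to the HUD's kill log box.
; The others call T7_GameStateBase to add random score, add a kill, or push hardcoded rifle and pistol weapon info.
; A disconnected branch for reading the player's current weapon never runs.
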(event Input|KeyboardEvents|DebugKey1
  (params (Key :type Key%20Structure :default "None") (ActionValue :type Input%20Action%20Value%20Structure))
  (bind _returnvalue (Game|Player|GetPlayerPawn 0))
  (:Pressed
    (bind _aswbp_hud (Utilities|Casting|CastToWBP_HUD2 (Class|T7PlayerController|GetHUDWidget)))
    (bind _asbp_player (Utilities|Casting|CastToBP_Player _returnvalue))
    (bind _returnvalue_2 (UserInterface|CreateWidget "/Game/UI/WBP_KillLog.WBP_KillLog_C" 0 (Utilities|Text|ToText(Object) _returnvalue) (Utilities|Text|ToText(Object) _returnvalue) "/Game/UI/Weapon_AR.Weapon_AR"))
    (Widget|Panel|AddChild (Variables|/Game/UI/WBP_HUD2.WBP_HUD2_C|GetKillLogBox _aswbp_hud) _returnvalue_2)))

(event Input|KeyboardEvents|DebugKey2
  (params (Key :type Key%20Structure :default "None") (ActionValue :type Input%20Action%20Value%20Structure))
  (:Pressed
    (bind _ast7_game_state_base (Utilities|Casting|CastToT7_GameStateBase (Game|GetGameState)))
    (Class|T7GameStateBase|AddScore _ast7_game_state_base (Math|Random|RandomIntegerinRange 1 99))))

(event Input|KeyboardEvents|DebugKey3
  (params (Key :type Key%20Structure :default "None") (ActionValue :type Input%20Action%20Value%20Structure))
  (:Pressed
    (bind _ast7_game_state_base (Utilities|Casting|CastToT7_GameStateBase (Game|GetGameState)))
    (Class|T7GameStateBase|AddKill _ast7_game_state_base 1)))

(event Input|KeyboardEvents|DebugKey4
  (params (Key :type Key%20Structure :default "None") (ActionValue :type Input%20Action%20Value%20Structure))
  (:Pressed
    (bind _ast7_game_state_base (Utilities|Casting|CastToT7_GameStateBase (Game|GetGameState)))
    (Class|T7GameStateBase|UpdateWeaponInfo _ast7_game_state_base "/Game/UI/Weapon_AR.Weapon_AR" "Assault Rifle" 30 120)))

(event Input|KeyboardEvents|DebugKey5
  (params (Key :type Key%20Structure :default "None") (ActionValue :type Input%20Action%20Value%20Structure))
  (:Pressed
    (bind _ast7_game_state_base (Utilities|Casting|CastToT7_GameStateBase (Game|GetGameState)))
    (Class|T7GameStateBase|UpdateWeaponInfo _ast7_game_state_base "/Game/UI/Weapon_Pistol.Weapon_Pistol" "Pistol" 7 21)))

(fn ConstructionScript)